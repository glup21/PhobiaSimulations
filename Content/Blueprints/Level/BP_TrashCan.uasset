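; BP_TrashCan is a puzzle receptacle that opens a linked Door once all actors tagged "Trackable" are inside its Box trigger.
; On BeginPlay it caches every tagged actor, then Box overlap events add and remove them from a Cubes collection, printing each change.
; When the Cubes count equals the cached total, it calls Open on the Door and sets Opened, so later overlaps are ignored.
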(event `self.ReceiveBeginPlay`
  (bind _outactors (`GameplayStatics.GetAllActorsWithTag` "Trackable"))
  (set `self.AllCubes` _outactors))

(event `self.Box.OnComponentBeginOverlap`
  (params (OverlappedComponent :type "PrimitiveComponent Object Reference") (OtherActor :type "Actor Object Reference") (OtherComp :type "PrimitiveComponent Object Reference") (OtherBodyIndex :type Integer) (bFromSweep :type Boolean) (SweepResult :type "HitResult Structure (by ref)"))
  (if (and (not (`self.Opened`)) (`self.ActorHasTag` OtherActor "Trackable"))
    (`KismetArrayLibrary.Array_Add` (`self.Cubes`) OtherActor)
    (`KismetSystemLibrary.PrintString` "Added")
    (if (== (`KismetArrayLibrary.Array_Length` (`self.Cubes`)) (`KismetArrayLibrary.Array_Length` (`self.AllCubes`)))
      (`/Game/Blueprints/Level/BP_Door.Open` (`self.Door`))
      (set `self.Opened` true))))

(event `self.Box.OnComponentEndOverlap`
  (params (OverlappedComponent :type "PrimitiveComponent Object Reference") (OtherActor :type "Actor Object Reference") (OtherComp :type "PrimitiveComponent Object Reference") (OtherBodyIndex :type Integer))
  (if (and (not (`self.Opened`)) (`self.ActorHasTag` OtherActor "Trackable"))
    (`KismetArrayLibrary.Array_RemoveItem` (`self.Cubes`) OtherActor)
    (`KismetSystemLibrary.PrintString` "Removed")))

(fn `UserConstructionScript`)