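; BP_SmallLamp is a small lamp Blueprint for levels, built around a point light.
; Its construction script copies the Intensity, LightColor and AttenuationRadius variables onto the light, so changes to them apply when the actor is constructed.
; The event graph holds only disabled default events, so the lamp has no runtime logic of its own.
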(fn `UserConstructionScript`
  (bind _pointlight (`self.PointLight`))
  (`LightComponent.SetIntensity` _pointlight (`self.Intensity`))
  (`LightComponent.SetLightColor` _pointlight (`self.LightColor`) true)
  (`LocalLightComponent.SetAttenuationRadius` (`self.PointLight`) (`self.AttenuationRadius`))
  (`LocalLightComponent.SetAttenuationRadius` _pointlight (`self.AttenuationRadius`)))