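; BP_StartTracking is a level trigger that starts data collection on the XR pawn and opens a door after a countdown.
; When a BP_XRPawn overlaps its box, it sets the pawn's IsCollectingData flag and starts the timer.
; Tick counts CurrentTime down by delta seconds, then calls Open on the referenced Door and destroys the trigger once it reaches zero.
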(event `self.ReceiveTick`
  (params (DeltaSeconds :type "Float (single-precision)"))
  (if (`self.TimerStarted`)
    (bind _output_get (set `self.CurrentTime` (- (`self.CurrentTime`) DeltaSeconds)))
    (if (<= _output_get 0.0)
      (`/Game/Blueprints/Level/BP_Door.Open` (`self.Door`))
      (`self.K2_DestroyActor`))))

(event `self.Box.OnComponentBeginOverlap`
  (params (OverlappedComponent :type "PrimitiveComponent Object Reference") (OtherActor :type "Actor Object Reference") (OtherComp :type "PrimitiveComponent Object Reference") (OtherBodyIndex :type Integer) (bFromSweep :type Boolean) (SweepResult :type "HitResult Structure (by ref)"))
  (bind _asbp_xrpawn (cast `/Game/XRFramework/Blueprints/BP_XRPawn` OtherActor))
  (set `/Game/XRFramework/Blueprints/BP_XRPawn.IsCollectingData` true _asbp_xrpawn)
  (set `self.TimerStarted` true))

(fn `UserConstructionScript`)