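; BP_MathTest is a level actor that runs a timed-seeded addition quiz through a floating UI spawned at its transform.
; On BeginPlay it finds the WB_MathQuestion widget inside the master widget's switcher, binds its answer event and seeds a random stream from time of day.
; Each submission prints correct or wrong feedback, then generates the next random sum until QuestionCount runs out.
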(event `MathAnswerSubmitted`
  (params (Answer :type Integer))
  (bind (_current_math_question_leftfactor _current_math_question_operator _current_math_question_rightfactor _current_math_question_answer) (break `/Game/Blueprints/Struct/BP_MathQuestion` (`self.Current Math Question`)))
  (`KismetSystemLibrary.PrintString` (`KismetStringLibrary.Conv_IntToString` Answer))
  (if (== Answer _current_math_question_answer)
    (`KismetSystemLibrary.PrintString` "Correct!" true true (struct :`R` 0.117788 :`G` 1.0 :`A` 1.0))
    (else
      (`KismetSystemLibrary.PrintString` "Wrong!!!" true true (struct :`R` 1.0 :`G` 0.007353 :`B` 0.000356 :`A` 1.0))))
  (`self.ConductMathTest`))

(event `self.ReceiveBeginPlay`
  (bind _returnvalue (`|SpawnActorFromClass` "/Game/Blueprints/UI/BP_FloatingUI.BP_FloatingUI_C" (`self.GetTransform`) "Undefined" "MultiplyWithRoot" null null))
  (bind _aswb_master_widget (cast `/Game/Blueprints/UI/WB_MasterWidget` (`WidgetComponent.GetWidget` (`/Game/Blueprints/UI/BP_FloatingUI.Widget` _returnvalue))))
  (bind _aswb_math_question (cast `/Game/Blueprints/UI/WB_MathQuestion` (`WidgetSwitcher.GetActiveWidget` (`/Game/Blueprints/UI/WB_MasterWidget.WidgetSwitcher_0` _aswb_master_widget))))
  (bind _output_get (set `self.As WB Math Question` _aswb_math_question))
  (add `/Game/Blueprints/UI/WB_MathQuestion.AnswerSubmitted` _output_get (delegate `MathAnswerSubmitted`))
  (set `self.RandomStream` (`KismetMathLibrary.MakeRandomStream` (`KismetMathLibrary.FTrunc` (`KismetMathLibrary.GetTotalSeconds` (`KismetMathLibrary.GetTimeOfDay` (struct))))))
  (`self.ConductMathTest`))

(event `ConductMathTest`
  (if (> (`self.QuestionCount`) 0)
    (bind _mathquestion (`self.GenerateMathQuestion`))
    (bind _output_get (set `self.Current Math Question` _mathquestion))
    (`/Game/Blueprints/UI/WB_MathQuestion.SetQuestion` (`self.As WB Math Question`) (`KismetStringLibrary.Concat_StrStr` (`KismetStringLibrary.Conv_IntToString` (break `/Game/Blueprints/Struct/BP_MathQuestion` _output_get)) "" (`.Operator_5_AD23E6A840955D7574B1898EE5FF01A4` (break `/Game/Blueprints/Struct/BP_MathQuestion` _output_get)) " " (`KismetStringLibrary.Conv_IntToString` (`.RightFactor_8_5EF350BD465C0233AC96918EE8B31B20` (break `/Game/Blueprints/Struct/BP_MathQuestion` _output_get))) "" "="))
    (`/Engine/EditorBlueprintResources/StandardMacros.DecrementInt` (`self.QuestionCount`))
    (else
      (`KismetSystemLibrary.PrintString` "Test ended!"))))

(fn `GenerateMathQuestion`
  (returns (MathQuestion :type "/Game/Blueprints/Struct/BP_MathQuestion Structure"))
  (locals (Operators :type "Array of String"))
  (bind _returnvalue (`KismetMathLibrary.RandomIntegerInRangeFromStream` (`self.RandomStream`) 0 (`self.MaxMathFactorValue`)))
  (bind _returnvalue_2 (`KismetMathLibrary.RandomIntegerInRangeFromStream` (`self.RandomStream`) 0 (`self.MaxMathFactorValue`)))
  (return (make `/Game/Blueprints/Struct/BP_MathQuestion` _returnvalue_2 "+" _returnvalue (+ _returnvalue_2 _returnvalue))))

(fn `UserConstructionScript`)