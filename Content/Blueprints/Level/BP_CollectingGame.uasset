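; BP_CollectingGame is a collecting minigame that starts on StartPlay and spawns one collectible at a time at randomly picked spawn points.
; When the current collectible overlaps the Box, it is destroyed and the next one spawns until CollectingCount is reached.
; On completion it prints a win message, spawns BP_MathTest at MathGameSpawnPosition and destroys itself, chaining into the next game.
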(event `StartPlay`
  (set `self.IsPlaying` true)
  (`self.SpawnNewCollectible`))

(event `self.Box.OnComponentBeginOverlap`
  (params (OverlappedComponent :type "PrimitiveComponent Object Reference") (OtherActor :type "Actor Object Reference") (OtherComp :type "PrimitiveComponent Object Reference") (OtherBodyIndex :type Integer) (bFromSweep :type Boolean) (SweepResult :type "HitResult Structure (by ref)"))
  (if (and (== (`self.CurrentCollectible`) OtherActor) (`self.IsPlaying`))
    (`self.K2_DestroyActor` (`self.CurrentCollectible`))
    (if (== (`self.CurrentCount`) (`self.CollectingCount`))
      (`KismetSystemLibrary.PrintString` "You won!")
      (`|SpawnActorFromClass` "/Game/Blueprints/Level/BP_MathTest.BP_MathTest_C" (`self.GetTransform` (`self.MathGameSpawnPosition`)) "Undefined" "MultiplyWithRoot" null null)
      (`self.K2_DestroyActor`)
      (else
        (`self.SpawnNewCollectible`)))))

(fn `Play`)

(fn `SpawnNewCollectible`
  (bind _spawnpoints (`self.SpawnPoints`))
  (bind (_returnvalue_location _returnvalue_rotation) (`KismetMathLibrary.BreakTransform` (`self.GetTransform` (`|GetArrayItem` _spawnpoints (`KismetMathLibrary.RandomIntegerInRange` 0 (`KismetArrayLibrary.Array_Length` _spawnpoints))))))
  (bind _returnvalue (`|SpawnActorFromClass` (`self.Collectible`) (`KismetMathLibrary.MakeTransform` _returnvalue_location _returnvalue_rotation) "Undefined" "MultiplyWithRoot" null null))
  (set `self.CurrentCollectible` _returnvalue)
  (`/Engine/EditorBlueprintResources/StandardMacros.IncrementInt` (`self.CurrentCount`)))

(fn `UserConstructionScript`)